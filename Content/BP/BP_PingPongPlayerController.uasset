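; Player controller for the ping pong game that toggles two selection menus from the keyboard.
; M alternates between showing and removing the map selection widget, and Tab does the same for the DLC selection widget.
; Each FlipFlop creates a fresh widget on open, stores its reference, shows the mouse cursor, and removes the widget and hides the cursor on close.
; The two toggles are independent and input mode is never changed.
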(event `Key|M`
  (params (Key :type "Key Structure"))
  (bind _mapselectionwidgetref (`self.MapSelectionWidgetRef`))
  (:`Pressed`
    (`/Engine/EditorBlueprintResources/StandardMacros.FlipFlop`
      (:`A`
        (bind _returnvalue (`|CreateWidget` "/Game/UI/WBP_MapSelectionWidget.WBP_MapSelectionWidget_C" self))
        (bind _output_get (set `self.MapSelectionWidgetRef` _returnvalue))
        (`UserWidget.AddToViewport` _output_get 0)
        (set `self.bShowMouseCursor` true))
      (:`B`
        (`/Engine/EditorBlueprintResources/StandardMacros.IsValid` _mapselectionwidgetref
          (:`Is Valid`
            (`Widget.RemoveFromParent` _mapselectionwidgetref)
            (set `self.bShowMouseCursor` false)))))))

(event `Key|Tab`
  (params (Key :type "Key Structure"))
  (bind _objectselectionwidgetref (`self.ObjectSelectionWidgetRef`))
  (:`Pressed`
    (`/Engine/EditorBlueprintResources/StandardMacros.FlipFlop`
      (:`A`
        (bind _returnvalue (`|CreateWidget` "/Game/UI/WBP_DLCSelectionWidget.WBP_DLCSelectionWidget_C" self))
        (bind _output_get (set `self.ObjectSelectionWidgetRef` _returnvalue))
        (`UserWidget.AddToViewport` _output_get 0)
        (set `self.bShowMouseCursor` true))
      (:`B`
        (`/Engine/EditorBlueprintResources/StandardMacros.IsValid` _objectselectionwidgetref
          (:`Is Valid`
            (`Widget.RemoveFromParent` _objectselectionwidgetref)
            (set `self.bShowMouseCursor` false)))))))

(fn `UserConstructionScript`)